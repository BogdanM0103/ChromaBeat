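; BP_TrackGenerator builds a track of event actors from the Elephant_track data table.
; Generate first runs ClearTrack, which destroys the attached actors, then looks up each row's Event in the EventClasses map.
; Each match spawns at the row's distance (X) and lane (Y), with X scale derived from Length.
; Spawned actors attach to the generator, so the next clear removes them.
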(event `Clear Track`
  (for _array_element (`self.GetAttachedActors` true)
    (`self.K2_DestroyActor` _array_element)))

(event `Generate`
  (`self.Clear Track`)
  (bind _outrownames (`DataTableFunctionLibrary.GetDataTableRowNames` "/Game/Data_Elephant/elephant_track.elephant_track"))
  (for _array_element _outrownames
    (bind _returnvalue (`|GetDataTableRow` "/Game/Data_Elephant/elephant_track.elephant_track" _array_element)
      (:`then`
        (bind (_time _distancex _laneindex _laney _event _strength _section _length) (break `/Game/Data_Elephant/S_TrackEvent` _returnvalue))
        (bind (_value _returnvalue_2) (`BlueprintMapLibrary.Map_Find` (`self.EventClasses`) _event))
        (if _returnvalue_2
          (bind _returnvalue_3 (`|SpawnActorFromClass` _value (`KismetMathLibrary.MakeTransform` (`KismetMathLibrary.MakeVector` _distancex _laney) (struct) (`KismetMathLibrary.MakeVector` (/ _length 100.0) 1.0 1.0)) "AlwaysSpawn" "MultiplyWithRoot" null null))
          (`self.K2_AttachToActor` _returnvalue_3 self "None" "KeepWorld" "KeepWorld" "KeepWorld" true))))))

(fn `UserConstructionScript`)