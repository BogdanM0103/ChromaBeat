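; BP_Conductor is a rhythm-timing actor that plays the song and exposes its position and beat length.
; One second after BeginPlay, StartSong records the audio-clock start time and plays MusicComp.
; GetSongPosition derives time from that clock, corrected for first-beat and latency offsets, returning a sentinel when not playing.
; Tick runs a test metronome that advances LastBeatIndex using BPM-derived beat length, without triggering anything else.
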(event `self.ReceiveBeginPlay`
  ;[0 0.4522 0.4983 0.5] Starts song when play is pressed
  (`KismetSystemLibrary.Delay` 1.0)
  (`self.StartSong`))

(event `self.ReceiveTick`
  (params (DeltaSeconds :type "Float (single-precision)"))
  (bind _returnvalue (`KismetMathLibrary.FFloor` (/ (`self.GetSongPosition`) (`self.GetSecondsPerBeat`))))
  ;[0.04413 0.4252 0.467 0.5] Test metronome
  (if (`self.isPlaying`)
    (if (> _returnvalue (`self.LastBeatIndex`))
      (set `self.LastBeatIndex` _returnvalue))))

(fn `GetSecondsPerBeat`
  (returns (Seconds :type "Float (double-precision)"))
  ;[0.15 0.0218 0.1351 0.5] Returns the duration of one beat in seconds (60 / BPM)
  (return (`KismetMathLibrary.SafeDivide` 60.0 (`self.BPM`))))

(fn `GetSongPosition`
  (returns (Position :type "Float (double-precision)"))
  ;[0.142 0.03102 0.15 0.5] Returns the current song position in seconds, relative to the first beat. Returns -9999 if the song hasn’t started
  (return (`KismetMathLibrary.SelectFloat` (- (- (- (`GameplayStatics.GetAudioTimeSeconds`) (`self.SongStartTime`)) (`self.FirstBeatOffset`)) (`self.AudioLatencyOffset`)) -9999.0 (`self.isPlaying`))))

(fn `StartSong`
  ;[0.15 0.03272 0.1496 0.5] Starts the music and stores the start time. Call once at the beginning of the level
  (set `self.SongStartTime` (`GameplayStatics.GetAudioTimeSeconds`))
  (set `self.isPlaying` true)
  (`AudioComponent.Play` (`self.MusicComp`) 0.0))

(fn `UserConstructionScript`)