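; BP_Note is a rhythm game note that travels along the Y axis toward a hit point in time with the song.
; Each tick it derives its position from the Conductor's song position, so movement follows the music rather than speed.
; Past the miss window it notifies the Conductor once, then destroys itself further beyond the hit point.
; BreakNote spawns a Niagara burst and scales the note up during a short remaining lifespan.
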(event `self.ReceiveTick`
  (params (DeltaSeconds :type "Float (single-precision)"))
  (bind _returnvalue (* (`GameplayStatics.GetWorldDeltaSeconds`) 6.0))
  ;[0.04792 0.1204 0.15 0.5] Move note towards player (time-based) and check if a note passed the player (miss)
  (if (`self.isHit`)
    (`self.SetActorScale3D` (+ (`self.GetActorScale3D`) (`KismetMathLibrary.MakeVector` _returnvalue _returnvalue _returnvalue)))
    (else
      (`/Engine/EditorBlueprintResources/StandardMacros.IsValid` (`self.Conductor`)
        (:`Is Valid`
          (set `self.Alpha` (/ (- (`self.NoteTime`) (`/Game/Blueprints/Breakables/BP_Conductor.GetSongPosition` (`self.Conductor`))) (`self.TravelTime`)))
          (`self.K2_SetActorLocation` (+ (`KismetMathLibrary.MakeVector` 0.0 (* (`self.Alpha`) (`self.SpawnDistance`))) (`self.HitPoint`)))
          (`|ExecutionSequence`
            (:`then_0`
              (if (and (> (- (`/Game/Blueprints/Breakables/BP_Conductor.GetSongPosition` (`self.Conductor`)) (`self.NoteTime`)) (`self.MissWindow`)) (not (`self.isMissed`)))
                (set `self.isMissed` true)
                (`/Game/Blueprints/Breakables/BP_Conductor.OnNoteMissed` (`self.Conductor`) (`self.K2_GetActorLocation`))))
            (:`then_1`
              (if (< (`self.Alpha`) -0.5)
                (`self.K2_DestroyActor`)))))))))

(event `BreakNote`
  ;[0.15 0.01982 0.02613 0.5] Particle Effect for hitting a note on time
  (set `self.isHit` true)
  (`self.SetLifeSpan` 0.15)
  (`NiagaraFunctionLibrary.SpawnSystemAtLocation` "/Game/Blueprints/Breakables/NS_NoteHit.NS_NoteHit" (`self.K2_GetActorLocation`)))

(fn `UserConstructionScript`)