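; Rhythm note spawner that feeds BP_Note actors from NoteTable in time with the song.
; On BeginPlay it finds BP_Conductor as the song clock and caches the table's row names.
; Each tick it converts the next row's beat to seconds and, TravelTime ahead of it, spawns at most one note offset along Y by SpawnDistance.
; Each note receives its timing, type, conductor and the spawner's location as HitPoint.
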(event `self.ReceiveBeginPlay`
  ;[0.04087 0.1233 0.1124 0.8087] Setup: find the song clock and load the note list
  (bind _returnvalue (`GameplayStatics.GetActorOfClass` "/Game/Blueprints/Breakables/BP_Conductor.BP_Conductor_C"))
  (set `self.Conductor` _returnvalue)
  (bind _outrownames (`DataTableFunctionLibrary.GetDataTableRowNames` (`self.NoteTable`)))
  (set `self.RowNames` _outrownames))

(event `self.ReceiveTick`
  (params (DeltaSeconds :type "Float (single-precision)"))
  (bind _returnvalue (`self.K2_GetActorLocation`))
  (bind _conductor (`self.Conductor`))
  ;[0.04036 0.148 0.15 0.5] Each tick: reads the next note from NoteTable and spawns it TravelTime seconds before its beat, so it arrives at HitPoint exactly on the beat. One note per tick
  (if (< (`self.NextNoteIndex`) (`KismetArrayLibrary.Array_Length` (`self.RowNames`)))
    (bind _returnvalue_2 (`|GetDataTableRow` (`self.NoteTable`) (`|GetArrayItem` (`self.RowNames`) (`self.NextNoteIndex`)))
      (:`then`
        (bind (_beatnumber _notetype) (break `/Game/Blueprints/Breakables/S_NoteData` _returnvalue_2))
        (set `self.NoteTime` (* _beatnumber (`/Game/Blueprints/Breakables/BP_Conductor.GetSecondsPerBeat` _conductor)))
        (if (>= (`/Game/Blueprints/Breakables/BP_Conductor.GetSongPosition` (`self.Conductor`)) (- (`self.NoteTime`) (`self.TravelTime`)))
          (`|SpawnActorFromClass` "/Game/Blueprints/Breakables/BP_Note.BP_Note_C" (`KismetMathLibrary.MakeTransform` (+ _returnvalue (`KismetMathLibrary.MakeVector` 0.0 (`self.SpawnDistance`)))) "Undefined" "MultiplyWithRoot" null (`self.NoteTime`) _returnvalue _conductor (`self.TravelTime`) (`self.SpawnDistance`) _notetype null)
          (set `self.NextNoteIndex` (+ (`self.NextNoteIndex`) 1)))))))

(fn `UserConstructionScript`)