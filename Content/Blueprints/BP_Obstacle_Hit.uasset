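; BP_Obstacle_Hit is a runner obstacle that penalizes the player for leaving it behind.
; Each Tick it compares the player character's X location with its own.
; Once the player is more than 200 units ahead, it calls LoseLife on BP_Runner, prints a MISS message and destroys itself.
; It has no overlap or hit handling of its own.
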(event `self.ReceiveTick`
  (params (DeltaSeconds :type "Float (single-precision)"))
  (bind _returnvalue (`GameplayStatics.GetPlayerCharacter` 0))
  (if (> (- (.x (`self.K2_GetActorLocation` _returnvalue)) (.x (`self.K2_GetActorLocation`))) 200.0)
    (bind _asbp_runner (cast `/Game/Blueprints/BP_Runner` _returnvalue))
    (`/Game/Blueprints/BP_Runner.LoseLife` _asbp_runner)
    (`KismetSystemLibrary.PrintString` "MISS" true true (struct :`R` 1.0 :`G` 0.15 :`B` 0.15 :`A` 1.0) 0.6 "judge")
    (`self.K2_DestroyActor`)))

(fn `UserConstructionScript`)